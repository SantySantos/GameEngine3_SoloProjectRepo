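; Base enemy character that provides the movement, patrol and spear combat actions.
; WieldSpear spawns a BP_Spear attached to the right-hand socket, and Attack plays a montage that calls OnAttackEnd whether completed or interrupted.
; It also exposes its patrol route and maps a speed state from idle to sprinting onto the max walk speed.
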(event `self.ReceiveBeginPlay`)

(event `WieldSpear`
  (bind _returnvalue (`|SpawnActorFromClass` "/Game/Blueprints/AI/Weapons/BP_Spear.BP_Spear_C" (`KismetMathLibrary.MakeTransform` (0.0 0.0 0.0)) "Undefined" "MultiplyWithRoot" self null))
  (`self.K2_AttachToComponent` _returnvalue (`self.Mesh`) "hand_r_sword_socket" "SnapToTarget" "SnapToTarget" "SnapToTarget" true)
  (set `self.isWieldingSpear` true))

(event `Attack`
  (`|PlayMontage` (`self.Mesh`) "/Game/Fab/SpearAnimationsV2/Animations/Character/1Hand/Pose02/Montage_BasicAttack.Montage_BasicAttack"
    (:`OnCompleted`
      _)
    (:`OnInterrupted`
      _))
  (`self.onAttackEnd`))

(fn `GetPatrolRoute`
  (returns (PatrolRoute :type "/Game/Blueprints/AI/BP_PatrolRoute Object Reference"))
  (return (`self.PatrolRoute`)))

(fn `SetMovementSpeed`
  (params (Speed :type "/Game/Blueprints/AI/Enums/E_MovementSpeed Enum" :default "NewEnumerator0"))
  (returns (SpeedValue :type "Float (double-precision)"))
  (bind _output_get (set `CharacterMovementComponent.MaxWalkSpeed` (select `/Game/Blueprints/AI/Enums/E_MovementSpeed` Speed :`NewEnumerator1` 100.0 :`NewEnumerator2` 300.0 :`NewEnumerator3` 500.0 :!type "Float (single-precision)") (`self.CharacterMovement`)))
  (return _output_get))

(fn `UserConstructionScript`)