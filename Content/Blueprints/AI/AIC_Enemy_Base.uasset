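; Base AI controller for enemies that drives their behavior through the BT_Enemy_Base behavior tree.
; On possession it starts the tree and puts the enemy into a passive state.
; SetStateAsPassive and SetStateAsAttacking write an E_AIState value to the blackboard, and the attacking variant also stores the target actor to attack.
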(event `self.ReceivePossess`
  (params (PossessedPawn :type "Pawn Object Reference"))
  ; Run before begin play
  (`self.RunBehaviorTree` "/Game/Blueprints/AI/BT_Enemy_Base.BT_Enemy_Base")
  (`self.SetStateAsPassive`))

(fn `SetStateAsAttacking`
  (params (AttackTarget :type "Actor Object Reference"))
  (`BlackboardComponent.SetValueAsObject` (`self.Blackboard`) (`self.TargetAttackKeyName`) AttackTarget)
  (`BlackboardComponent.SetValueAsEnum` (`self.Blackboard`) (`self.State Key Name`) (enumliteral `/Game/Blueprints/AI/Enums/E_AIState` "NewEnumerator1")))

(fn `SetStateAsPassive`
  (`BlackboardComponent.SetValueAsEnum` (`self.Blackboard`) (`self.State Key Name`) (enumliteral `/Game/Blueprints/AI/Enums/E_AIState` "NewEnumerator0")))

(fn `UserConstructionScript`)