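; BP_Turret is a mountable turret that a BP_ThirdPersonCharacter can enter, aim and fire.
; Sphere overlap stores the player, adds IMC_Turret and enables input, which is disabled again on dismount.
; The use action flip-flops between seating the player with a camera blend to the turret and restoring their saved location and view.
; While manned, Tick follows control rotation with clamped pitch, and the fire action spawns BP_Projectile at the Nozzle.
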(event `self.ReceiveTick`
  (params (DeltaSeconds :type "Float (single-precision)"))
  (bind _returnvalue_roll (`KismetMathLibrary.BreakRotator` (`self.K2_GetActorRotation`)))
  (bind _owningplayer (`self.OwningPlayer`))
  (bind (_returnvalue_roll_2 _returnvalue_pitch _returnvalue_yaw) (`KismetMathLibrary.BreakRotator` (`Pawn.GetControlRotation` _owningplayer)))
  (`/Engine/EditorBlueprintResources/StandardMacros.IsValid` _owningplayer
    (:`Is Valid`
      (if (`TP_ThirdPersonCharacter.bInTurret` _owningplayer)
        (`self.K2_SetActorRotation` (`KismetMathLibrary.MakeRotator` _returnvalue_roll (`KismetMathLibrary.ClampAngle` _returnvalue_pitch -45.0 45.0) _returnvalue_yaw))))))

(event `self.Sphere.OnComponentBeginOverlap`
  (params (OverlappedComponent :type "PrimitiveComponent Object Reference") (OtherActor :type "Actor Object Reference") (OtherComp :type "PrimitiveComponent Object Reference") (OtherBodyIndex :type Integer) (bFromSweep :type Boolean) (SweepResult :type "HitResult Structure (by ref)"))
  (bind _asbp_third_person_character (cast `/Game/ThirdPerson/Blueprints/BP_ThirdPersonCharacter` OtherActor))
  (set `self.OwningPlayer` _asbp_third_person_character)
  (bind _asplayer_controller (cast `PlayerController` (`Pawn.GetController` (`self.OwningPlayer`))))
  (bind _returnvalue (pcsubsystem `EnhancedInputLocalPlayerSubsystem` _asplayer_controller))
  (`/Engine/EditorBlueprintResources/StandardMacros.IsValid` _returnvalue
    (:`Is Valid`
      (`EnhancedInputSubsystemInterface.AddMappingContext` _returnvalue "/Game/Input/IMC_Turret.IMC_Turret" 1 (struct))
      (`self.EnableInput` _asplayer_controller))))

(event `EnhancedInput|/Game/Input/Actions/IA_FireTurret`
  (params (ActionValue :type Boolean) (ElapsedSeconds :type "Float (double-precision)") (TriggeredSeconds :type "Float (double-precision)") (InputAction :type "InputAction Object Reference" :default "/Game/Input/Actions/IA_FireTurret.IA_FireTurret"))
  (:`Started`
    (if (`TP_ThirdPersonCharacter.bInTurret` (`self.OwningPlayer`))
      (`|SpawnActorFromClass` "/Game/Blueprints/BP_Projectile.BP_Projectile_C" (`KismetMathLibrary.MakeTransform` (`SceneComponent.K2_GetComponentLocation` (`self.Nozzle`)) (`self.K2_GetActorRotation`)) "Undefined" "MultiplyWithRoot" self null)
      (`AudioComponent.Play` (`self.Projectile`) 0.0))))

(event `EnhancedInput|/Game/Input/Actions/IA_UseTurret`
  (params (ActionValue :type Boolean) (ElapsedSeconds :type "Float (double-precision)") (TriggeredSeconds :type "Float (double-precision)") (InputAction :type "InputAction Object Reference" :default "/Game/Input/Actions/IA_UseTurret.IA_UseTurret"))
  (bind _owningplayer (`self.OwningPlayer`))
  (bind _owningplayer_2 (`self.OwningPlayer`))
  (bind _owningplayer_3 (`self.OwningPlayer`))
  (bind _owningplayer_4 (`self.OwningPlayer`))
  (:`Started`
    (`/Engine/EditorBlueprintResources/StandardMacros.IsValid` _owningplayer_4
      (:`Is Valid`
        (`/Engine/EditorBlueprintResources/StandardMacros.FlipFlop`
          (:`A`
            (set `self.LastPlayerLocation` (`self.K2_GetActorLocation` _owningplayer_4))
            (set `MovementComponent.Velocity` (0.0 0.0 0.0) (`Character.CharacterMovement` _owningplayer))
            (bind _asplayer_controller (cast `PlayerController` (`Pawn.GetController` _owningplayer)))
            (`PlayerController.SetViewTargetWithBlend` _asplayer_controller self 0.5 "VTBlend_Linear" 0.0 false)
            (set `TP_ThirdPersonCharacter.bInTurret` true _owningplayer_2)
            (`self.K2_SetActorRotation` _owningplayer_2 (`self.K2_GetActorRotation`) false)
            (`self.K2_AttachToComponent` _owningplayer_2 (`self.PlayerSeat`) "None" "SnapToTarget" "SnapToTarget" "KeepRelative" true))
          (:`B`
            (bind _asplayer_controller_2 (cast `PlayerController` (`Pawn.GetController` _owningplayer_4)))
            (`PlayerController.SetViewTargetWithBlend` _asplayer_controller_2 (`self.OwningPlayer`) 0.5 "VTBlend_Linear" 0.0 false)
            (`self.K2_DetachFromActor` _owningplayer_3 "KeepWorld" "KeepWorld" "KeepWorld")
            (`self.K2_SetActorLocation` _owningplayer_3 (`self.LastPlayerLocation`) false true)
            (set `TP_ThirdPersonCharacter.bInTurret` false _owningplayer_2)
            (`self.DisableInput` _asplayer_controller_2)))))))

(fn `UserConstructionScript`)