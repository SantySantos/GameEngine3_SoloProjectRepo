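; BP_Boss is a boss actor that takes damage from projectiles and tracks it through a BPHealthSystem component.
; BeginPlay sets a high maximum health on that component.
; On Hit, a BP_Projectile deals random integer damage through the component and is then destroyed.
; The Die event only prints a death message, with no further death handling.
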(event `self.ReceiveBeginPlay`
  (`/Game/Blueprints/BP_HealthSystem.SetMaxHealth` (`self.BP_HealthSystem`) 1000.0))

(event `self.ReceiveHit`
  (params (MyComp :type "PrimitiveComponent Object Reference") (Other :type "Actor Object Reference") (OtherComp :type "PrimitiveComponent Object Reference") (bSelfMoved :type Boolean) (HitLocation :type "Vector Structure") (HitNormal :type "Vector Structure") (NormalImpulse :type "Vector Structure") (Hit :type "HitResult Structure (by ref)"))
  (`KismetSystemLibrary.IsObjectOfSoftClass` Other "/Game/Blueprints/BP_Projectile.BP_Projectile_C"
    (:`True`
      (`/Game/Blueprints/BP_HealthSystem.TakeDamage` (`self.BP_HealthSystem`) (`KismetMathLibrary.Conv_IntToDouble` (`KismetMathLibrary.RandomIntegerInRange` 5 20)))
      (`self.K2_DestroyActor` Other))))

(event `/Game/Blueprints/BPI_Death.Die`
  (`KismetSystemLibrary.PrintString` "Boss is Death"))

(fn `UserConstructionScript`)