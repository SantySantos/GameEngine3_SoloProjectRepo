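; BP_Platform is a platform actor that takes over the player's view when the player character enters its sphere trigger.
; On overlap it prints a debug message, waits briefly, then blends the player controller's view target to itself.
; The construction script keeps the SpringArm at unit world scale.
; A PlatformAnim timeline would lerp the actor toward TargetPoint, but nothing starts it, so the platform does not move.
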(event `self.Sphere.OnComponentBeginOverlap`
  (params (OverlappedComponent :type "PrimitiveComponent Object Reference") (OtherActor :type "Actor Object Reference") (OtherComp :type "PrimitiveComponent Object Reference") (OtherBodyIndex :type Integer) (bFromSweep :type Boolean) (SweepResult :type "HitResult Structure (by ref)"))
  (if (== OtherActor (`GameplayStatics.GetPlayerCharacter` 0))
    (`KismetSystemLibrary.PrintString` "Collition detected")
    (`KismetSystemLibrary.Delay` 2.0)
    (`PlayerController.SetViewTargetWithBlend` (`GameplayStatics.GetPlayerController` 0) self 2.0 "VTBlend_Linear" 0.0 false)))

(fn `UserConstructionScript`
  (`SceneComponent.SetWorldScale3D` (`self.SpringArm`) (`KismetMathLibrary.Conv_IntToVector` 1)))