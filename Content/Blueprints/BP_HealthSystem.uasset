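; BP_HealthSystem is a health component that tracks damage and healing for its owning actor.
; Health starts at MaxHealth on BeginPlay, and healing is capped at that maximum.
; Damage subtracts from Health with debug prints of the owner's class, the amount and the remaining value.
; When Health drops to zero or below, it calls DieMessage on the owner, leaving death handling to that actor.
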(event `self.ReceiveBeginPlay`
  (`self.SetMaxHealth` (`self.MaxHealth`))
  (set `self.Health` (`self.MaxHealth`)))

(event `SetMaxHealth`
  (params (MaxHealth :type "Float (double-precision)"))
  (set `self.MaxHealth` MaxHealth))

(event `TakeDamage`
  (params (DamageAmount :type "Float (double-precision)"))
  (`KismetSystemLibrary.PrintString` (`KismetStringLibrary.Concat_StrStr` (`KismetStringLibrary.Concat_StrStr` (`KismetSystemLibrary.GetClassDisplayName` (`GameplayStatics.GetObjectClass` (`self.GetOwner`))) "took:") (`KismetStringLibrary.Conv_DoubleToString` DamageAmount)))
  (bind _output_get (set `self.Health` (- (`self.Health`) DamageAmount)))
  (`KismetSystemLibrary.PrintString` (`KismetStringLibrary.Conv_DoubleToString` _output_get) true true (struct :`R` 0.26407 :`G` 1.0 :`A` 1.0))
  (if (<= _output_get 0.0)
    (message `/Game/Blueprints/BPI_Death.Die` (`self.GetOwner`))))

(event `TakeHeal`
  (params (HealAmount :type "Float (double-precision)"))
  (bind _returnvalue (+ HealAmount (`self.Health`)))
  (if (<= _returnvalue (`self.MaxHealth`))
    (set `self.Health` _returnvalue)
    (else
      (set `self.Health` (`self.MaxHealth`)))))